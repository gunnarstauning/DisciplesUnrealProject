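; Coin item actor that shows a pickup prompt while the first-person character overlaps it.
; At BeginPlay it applies its ItemMesh variable to the DefaultCoin mesh component.
; Overlap begin finds all top-level PickupWidget instances, sets their item name from the Type enum and shows them, and overlap end hides them.
; The file contains no logic for collecting the coin.
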(event `self.ReceiveBeginPlay`
  (`StaticMeshComponent.SetStaticMesh` (`self.Default_Coin`) (`self.Item_Mesh`)))

(event `self.ReceiveActorBeginOverlap`
  (params (OtherActor :type "Actor Object Reference"))
  (cast `/Game/FirstPersonBP/Blueprints/FirstPersonCharacter` OtherActor)
  (bind _foundwidgets (`WidgetBlueprintLibrary.GetAllWidgetsOfClass` "/Game/PickupWidget.PickupWidget_C"))
  (for _array_element _foundwidgets
    (set `/Game/PickupWidget.ItemName` (`KismetTextLibrary.Conv_StringToText` (`|GetEnumeratorNameAsString` (`self.Type`))) _array_element)
    (`Widget.SetVisibility` _array_element "Visible")))

(event `self.ReceiveActorEndOverlap`
  (params (OtherActor :type "Actor Object Reference"))
  (cast `/Game/FirstPersonBP/Blueprints/FirstPersonCharacter` OtherActor)
  (bind _foundwidgets (`WidgetBlueprintLibrary.GetAllWidgetsOfClass` "/Game/PickupWidget.PickupWidget_C"))
  (for _array_element _foundwidgets
    (`Widget.SetVisibility` _array_element "Hidden")))

(fn `UserConstructionScript`)